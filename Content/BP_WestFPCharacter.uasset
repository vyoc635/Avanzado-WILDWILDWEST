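; BP_WestFPCharacter is a character Blueprint, first-person by its name, that provides basic walk and jump actions.
; Move applies a 2D input along the forward and right vectors of the Camera's yaw only, so pitch and roll do not affect movement.
; StartJump and StopJump wrap the built-in Jump and StopJumping.
; The event graph holds only disabled stubs and binds no input itself.
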(event EventBeginPlay)

(event Collision|EventActorBeginOverlap
  (params (OtherActor :type Actor%20Object%20Reference)))

(event EventTick
  (params (DeltaSeconds :type Float%20%28single-precision%29)))

(fn ConstructionScript)

(fn Move
  (params (Input :type Vector%202D%20Structure))
  (bind _camera (Variables|Default|GetCamera))
  (bind _returnvalue (Transformation|GetWorldRotation _camera))
  (bind _returnvalue_2 (Math|Rotator|MakeRotator 0.0 0.0 (.yaw _returnvalue)))
  (Pawn|Input|AddMovementInput (Math|Vector|GetRightVector _returnvalue_2) (.x Input) false)
  (Pawn|Input|AddMovementInput (Math|Vector|GetForwardVector _returnvalue_2) (.y Input) false))

(fn StartJump
  (Character|Jump))

(fn StopJump
  (Character|StopJumping))